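; BP_PlatfomTrap is a single-use trap in the car derby that damages the car overlapping it.
; On overlap it sorts AI sedans from player Sedans by cast and routes fixed damage through VehicleGameMode.
; An AI car left without HP is destroyed, while a player car is handed to the game mode's death-and-spectate function.
; The trap then destroys itself; a few unconnected debug and HP nodes remain unused.
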(event `self.ReceiveActorBeginOverlap`
  (params (OtherActor :type "Actor Object Reference"))
  (`parent.ReceiveActorBeginOverlap` OtherActor)
  (bind _asbp_sedan_ai (cast `/Game/CarDerby/AI/BP_Sedan_AI` OtherActor)
    (:`then`
      (bind _asvehicle_game_mode (cast `/Game/CarDerby/VehicleGameMode` (`GameplayStatics.GetGameMode`)))
      (`/Game/CarDerby/VehicleGameMode.AI_LostHP` _asvehicle_game_mode 30 _asbp_sedan_ai)
      (if (<= (`/Game/CarDerby/AI/BP_Sedan_AI.CurrentHP_MyCar` _asbp_sedan_ai) 0)
        (`self.K2_DestroyActor` _asbp_sedan_ai))
      (`self.K2_DestroyActor`))
    (:`CastFailed`
      (bind _assedan (cast `/Game/CarDerby/Sedan` OtherActor))
      (bind _asvehicle_game_mode_2 (cast `/Game/CarDerby/VehicleGameMode` (`GameplayStatics.GetGameMode`)))
      (`/Game/CarDerby/VehicleGameMode.PlayerLostHP_by_AI` _asvehicle_game_mode_2 30 _assedan)
      (if (<= (`/Game/CarDerby/Sedan.CurrentHP_MyCar` _assedan) 0)
        (bind _asvehicle_game_mode_3 (cast `/Game/CarDerby/VehicleGameMode` (`GameplayStatics.GetGameMode`)))
        (`/Game/CarDerby/VehicleGameMode.DethPlayerAndSpectate` _asvehicle_game_mode_3 _assedan))
      (`self.K2_DestroyActor`))))

(fn `UserConstructionScript`
  (`parent.UserConstructionScript`))