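; AI controller for car-derby sedans that drives a BP_Sedan_AI forward and chases its Target when one exists.
; Each Tick, Hunt steers by comparing yaw to an acos-derived bearing, split by the target's relative quadrant.
; DefinitingBlock line-traces ahead, turning away from obstacles while roaming; if nearly stopped against a hit, it sets Blocked to reverse until a timer clears it.
; AIMoveTo nodes are unconnected; movement uses direct MoveForward/MoveRight inputs.
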(event `self.ReceiveBeginPlay`
  (bind _asbp_sedan_ai (cast `/Game/CarDerby/AI/BP_Sedan_AI` (`self.K2_GetPawn`)))
  (set `self.OwnSedan AI` _asbp_sedan_ai))

(event `self.ReceiveTick`
  (params (DeltaSeconds :type "Float (single-precision)"))
  (if (`/Game/CarDerby/AI/BP_Sedan_AI.There_is_Target?` (`self.OwnSedan AI`))
    (`self.Hunt`)
    (if (`self.Blocked`)
      (`/Game/CarDerby/AI/BP_Sedan_AI.MoveForward` (`self.OwnSedan AI`) -1.0)
      (else
        (`self.DefinitingBlock`)))
    (elif (`self.Blocked`)
      (`/Game/CarDerby/AI/BP_Sedan_AI.MoveForward` (`self.OwnSedan AI`) -1.0)
      (else
        (`|ExecutionSequence`
          (:`then_0`
            (`self.DefinitingBlock`))
          (:`then_1`
            (`/Game/CarDerby/AI/BP_Sedan_AI.MoveForward` (`self.OwnSedan AI`) 1.0)))))))

(fn `DefinitingBlock`
  (bind _ownsedan_ai (`self.OwnSedan AI`))
  (bind _returnvalue (+ (`self.K2_GetActorLocation` _ownsedan_ai) (0.0 0.0 100.0)))
  (bind (_outhit _returnvalue_2) (`KismetSystemLibrary.LineTraceSingle` _returnvalue (+ _returnvalue (* (`self.GetActorForwardVector` _ownsedan_ai) 2500.0)) "TraceTypeQuery1" false (`|MakeArray` (`self.OwnSedan AI`) :!type "Actor Object Reference") "ForOneFrame"))
  (if (and (<= (`KismetMathLibrary.VSize` (`self.GetVelocity` (`self.OwnSedan AI`))) 2.0) _returnvalue_2)
    (if (`/Game/CarDerby/AI/BP_Sedan_AI.There_is_Target?` (`self.OwnSedan AI`))
      (set `self.Blocked` true)
      (`/Game/CarDerby/AI/BP_Sedan_AI.MoveRight` (`self.OwnSedan AI`) -1.0)
      (`KismetSystemLibrary.K2_SetTimer` null "ToggleBlock" 2.0)
      (else
        (set `self.Blocked` true)
        (`/Game/CarDerby/AI/BP_Sedan_AI.MoveRight` (`self.OwnSedan AI`) -1.0)
        (`KismetSystemLibrary.K2_SetTimer` null "ToggleBlock" 1.0)))
    (elif (`/Game/CarDerby/AI/BP_Sedan_AI.There_is_Target?` (`self.OwnSedan AI`))
      _
      (elif _returnvalue_2
        (`/Game/CarDerby/AI/BP_Sedan_AI.MoveRight` (`self.OwnSedan AI`) 1.0)
        (else
          (`/Game/CarDerby/AI/BP_Sedan_AI.MoveRight` (`self.OwnSedan AI`) 0.0))))))

(fn `Hunt`
  (bind _returnvalue_x (`KismetMathLibrary.BreakVector` (`self.K2_GetActorLocation` (`self.OwnSedan AI`))))
  (bind (_returnvalue_roll _returnvalue_pitch _returnvalue_yaw) (`KismetMathLibrary.BreakRotator` (`self.K2_GetActorRotation` (`self.OwnSedan AI`))))
  (bind _returnvalue_x_2 (`KismetMathLibrary.BreakVector` (`self.K2_GetActorLocation` (`self.OwnSedan AI`))))
  (bind (_returnvalue_x_3 _returnvalue_y) (`KismetMathLibrary.BreakVector` (`self.K2_GetActorLocation` (`self.OwnSedan AI`))))
  (bind (_returnvalue_x_4 _returnvalue_y_2) (`KismetMathLibrary.BreakVector` (`self.K2_GetActorLocation` (`self.OwnSedan AI`))))
  (bind (_returnvalue_roll_2 _returnvalue_pitch_2 _returnvalue_yaw_2) (`KismetMathLibrary.BreakRotator` (`self.K2_GetActorRotation` (`self.OwnSedan AI`))))
  (bind _returnvalue_x_5 (`KismetMathLibrary.BreakVector` (`self.K2_GetActorLocation` (`self.OwnSedan AI`))))
  (bind (_returnvalue_x_6 _returnvalue_y_3) (`KismetMathLibrary.BreakVector` (`self.K2_GetActorLocation` (`self.OwnSedan AI`))))
  (bind (_returnvalue_roll_3 _returnvalue_pitch_3 _returnvalue_yaw_3) (`KismetMathLibrary.BreakRotator` (`self.K2_GetActorRotation` (`self.OwnSedan AI`))))
  (bind (_returnvalue_roll_4 _returnvalue_pitch_4 _returnvalue_yaw_4) (`KismetMathLibrary.BreakRotator` (`self.K2_GetActorRotation` (`self.OwnSedan AI`))))
  (bind _returnvalue_x_7 (`KismetMathLibrary.BreakVector` (`self.K2_GetActorLocation` (`self.OwnSedan AI`))))
  (bind (_returnvalue_x_8 _returnvalue_y_4) (`KismetMathLibrary.BreakVector` (`self.K2_GetActorLocation` (`self.OwnSedan AI`))))
  (bind (_returnvalue_roll_5 _returnvalue_pitch_5 _returnvalue_yaw_5) (`KismetMathLibrary.BreakRotator` (`self.K2_GetActorRotation` (`self.OwnSedan AI`))))
  (bind _returnvalue_x_9 (`KismetMathLibrary.BreakVector` (`self.K2_GetActorLocation` (`self.OwnSedan AI`))))
  (bind (_returnvalue_x_10 _returnvalue_y_5) (`KismetMathLibrary.BreakVector` (`self.K2_GetActorLocation` (`self.OwnSedan AI`))))
  (bind _returnvalue_x_11 (`KismetMathLibrary.BreakVector` (`self.K2_GetActorLocation` (`self.OwnSedan AI`))))
  (bind (_returnvalue_x_12 _returnvalue_y_6) (`KismetMathLibrary.BreakVector` (`self.K2_GetActorLocation` (`self.OwnSedan AI`))))
  (bind (_returnvalue_roll_6 _returnvalue_pitch_6 _returnvalue_yaw_6) (`KismetMathLibrary.BreakRotator` (`self.K2_GetActorRotation` (`self.OwnSedan AI`))))
  (bind (_returnvalue_roll_7 _returnvalue_pitch_7 _returnvalue_yaw_7) (`KismetMathLibrary.BreakRotator` (`self.K2_GetActorRotation` (`self.OwnSedan AI`))))
  (bind (_returnvalue_roll_8 _returnvalue_pitch_8 _returnvalue_yaw_8) (`KismetMathLibrary.BreakRotator` (`self.K2_GetActorRotation` (`self.OwnSedan AI`))))
  (bind _returnvalue_x_13 (`KismetMathLibrary.BreakVector` (`self.K2_GetActorLocation` (`self.OwnSedan AI`))))
  (bind (_returnvalue_x_14 _returnvalue_y_7) (`KismetMathLibrary.BreakVector` (`self.K2_GetActorLocation` (`self.OwnSedan AI`))))
  (bind (_returnvalue_x_15 _returnvalue_y_8) (`KismetMathLibrary.BreakVector` (`self.K2_GetActorLocation` (`self.OwnSedan AI`))))
  (bind _returnvalue_x_16 (`KismetMathLibrary.BreakVector` (`self.K2_GetActorLocation` (`self.OwnSedan AI`))))
  (bind _returnvalue_x_17 (`KismetMathLibrary.BreakVector` (`self.K2_GetActorLocation` (`/Game/CarDerby/AI/BP_Sedan_AI.Target` (`self.OwnSedan AI`)))))
  (bind _returnvalue_x_18 (`KismetMathLibrary.BreakVector` (`self.K2_GetActorLocation` (`/Game/CarDerby/AI/BP_Sedan_AI.Target` (`self.OwnSedan AI`)))))
  (bind (_returnvalue_x_19 _returnvalue_y_9) (`KismetMathLibrary.BreakVector` (`self.K2_GetActorLocation` (`/Game/CarDerby/AI/BP_Sedan_AI.Target` (`self.OwnSedan AI`)))))
  (bind (_returnvalue_x_20 _returnvalue_y_10) (`KismetMathLibrary.BreakVector` (`self.K2_GetActorLocation` (`/Game/CarDerby/AI/BP_Sedan_AI.Target` (`self.OwnSedan AI`)))))
  (bind _returnvalue_x_21 (`KismetMathLibrary.BreakVector` (`self.K2_GetActorLocation` (`/Game/CarDerby/AI/BP_Sedan_AI.Target` (`self.OwnSedan AI`)))))
  (bind (_returnvalue_x_22 _returnvalue_y_11) (`KismetMathLibrary.BreakVector` (`self.K2_GetActorLocation` (`/Game/CarDerby/AI/BP_Sedan_AI.Target` (`self.OwnSedan AI`)))))
  (bind (_returnvalue_x_23 _returnvalue_y_12) (`KismetMathLibrary.BreakVector` (`self.K2_GetActorLocation` (`/Game/CarDerby/AI/BP_Sedan_AI.Target` (`self.OwnSedan AI`)))))
  (bind _returnvalue_x_24 (`KismetMathLibrary.BreakVector` (`self.K2_GetActorLocation` (`/Game/CarDerby/AI/BP_Sedan_AI.Target` (`self.OwnSedan AI`)))))
  (bind _returnvalue_x_25 (`KismetMathLibrary.BreakVector` (`self.K2_GetActorLocation` (`/Game/CarDerby/AI/BP_Sedan_AI.Target` (`self.OwnSedan AI`)))))
  (bind (_returnvalue_x_26 _returnvalue_y_13) (`KismetMathLibrary.BreakVector` (`self.K2_GetActorLocation` (`/Game/CarDerby/AI/BP_Sedan_AI.Target` (`self.OwnSedan AI`)))))
  (bind (_returnvalue_x_27 _returnvalue_y_14) (`KismetMathLibrary.BreakVector` (`self.K2_GetActorLocation` (`/Game/CarDerby/AI/BP_Sedan_AI.Target` (`self.OwnSedan AI`)))))
  (bind (_returnvalue_x_28 _returnvalue_y_15) (`KismetMathLibrary.BreakVector` (`self.K2_GetActorLocation` (`/Game/CarDerby/AI/BP_Sedan_AI.Target` (`self.OwnSedan AI`)))))
  (bind _returnvalue_x_29 (`KismetMathLibrary.BreakVector` (`self.K2_GetActorLocation` (`/Game/CarDerby/AI/BP_Sedan_AI.Target` (`self.OwnSedan AI`)))))
  (bind (_returnvalue_x_30 _returnvalue_y_16) (`KismetMathLibrary.BreakVector` (`self.K2_GetActorLocation` (`/Game/CarDerby/AI/BP_Sedan_AI.Target` (`self.OwnSedan AI`)))))
  (bind _returnvalue_x_31 (`KismetMathLibrary.BreakVector` (`self.K2_GetActorLocation` (`/Game/CarDerby/AI/BP_Sedan_AI.Target` (`self.OwnSedan AI`)))))
  (bind _returnvalue_x_32 (`KismetMathLibrary.BreakVector` (`self.K2_GetActorLocation` (`/Game/CarDerby/AI/BP_Sedan_AI.Target` (`self.OwnSedan AI`)))))
  (bind _returnvalue (- _returnvalue_x_18 _returnvalue_x_2))
  (bind _returnvalue_2 (- _returnvalue_x_5 _returnvalue_x_21))
  (bind _returnvalue_3 (- _returnvalue_x_7 _returnvalue_x_24))
  (bind _returnvalue_4 (- _returnvalue_x_9 _returnvalue_x_25))
  (bind _returnvalue_5 (- _returnvalue_x_31 _returnvalue_x_13))
  (bind _returnvalue_6 (- _returnvalue_x_32 _returnvalue_x_16))
  (bind _returnvalue_7 (/ _returnvalue (`KismetMathLibrary.VSize2D` (`KismetMathLibrary.MakeVector2D` _returnvalue (- _returnvalue_y _returnvalue_y_9)))))
  (bind _returnvalue_8 (/ _returnvalue_2 (`KismetMathLibrary.VSize2D` (`KismetMathLibrary.MakeVector2D` _returnvalue_2 (- _returnvalue_y_3 _returnvalue_y_11)))))
  (bind _returnvalue_9 (/ _returnvalue_3 (`KismetMathLibrary.VSize2D` (`KismetMathLibrary.MakeVector2D` _returnvalue_3 (- _returnvalue_y_4 _returnvalue_y_12)))))
  (bind _returnvalue_10 (/ _returnvalue_4 (`KismetMathLibrary.VSize2D` (`KismetMathLibrary.MakeVector2D` _returnvalue_4 (- _returnvalue_y_13 _returnvalue_y_5)))))
  (bind _returnvalue_11 (/ _returnvalue_6 (`KismetMathLibrary.VSize2D` (`KismetMathLibrary.MakeVector2D` _returnvalue_6 (- _returnvalue_y_8 _returnvalue_y_15)))))
  (bind _returnvalue_12 (/ _returnvalue_5 (`KismetMathLibrary.VSize2D` (`KismetMathLibrary.MakeVector2D` _returnvalue_5 (- _returnvalue_y_16 _returnvalue_y_7)))))
  (`/Game/CarDerby/AI/BP_Sedan_AI.MoveForward` (`self.OwnSedan AI`) 1.0)
  (if (> _returnvalue_x_11 _returnvalue_x_29)
    (if (< _returnvalue_y_2 _returnvalue_y_10)
      (if (< _returnvalue_yaw_5 (- 180.0 (`KismetMathLibrary.DegAcos` _returnvalue_10)))
        (`/Game/CarDerby/AI/BP_Sedan_AI.MoveRight` (`self.OwnSedan AI`) _returnvalue_10)
        (else
          (`/Game/CarDerby/AI/BP_Sedan_AI.MoveRight` (`self.OwnSedan AI`) (* _returnvalue_10 -1.0))))
      (elif (< _returnvalue_yaw_3 0.0)
        (if (< (+ 360.0 _returnvalue_yaw_4) (+ 180.0 (`KismetMathLibrary.DegAcos` _returnvalue_9)))
          (`/Game/CarDerby/AI/BP_Sedan_AI.MoveRight` (`self.OwnSedan AI`) _returnvalue_9)
          (else
            (`/Game/CarDerby/AI/BP_Sedan_AI.MoveRight` (`self.OwnSedan AI`) (* _returnvalue_9 -1.0))))
        (elif (< _returnvalue_yaw_2 (+ 180.0 (`KismetMathLibrary.DegAcos` _returnvalue_8)))
          (`/Game/CarDerby/AI/BP_Sedan_AI.MoveRight` (`self.OwnSedan AI`) _returnvalue_8)
          (else
            (`/Game/CarDerby/AI/BP_Sedan_AI.MoveRight` (`self.OwnSedan AI`) (* _returnvalue_8 -1.0))))))
    (elif (< _returnvalue_x _returnvalue_x_17)
      (if (< _returnvalue_y_6 _returnvalue_y_14)
        (if (> _returnvalue_yaw_8 (+ 0.0 (`KismetMathLibrary.DegAcos` _returnvalue_12)))
          (`/Game/CarDerby/AI/BP_Sedan_AI.MoveRight` (`self.OwnSedan AI`) (* _returnvalue_12 -1.0))
          (else
            (`/Game/CarDerby/AI/BP_Sedan_AI.MoveRight` (`self.OwnSedan AI`) _returnvalue_12)))
        (elif (< _returnvalue_yaw_7 0.0)
          (if (> (+ 0.0 _returnvalue_yaw_6) (- 0.0 (`KismetMathLibrary.DegAcos` _returnvalue_11)))
            (`/Game/CarDerby/AI/BP_Sedan_AI.MoveRight` (`self.OwnSedan AI`) (* _returnvalue_11 -1.0))
            (else
              (`/Game/CarDerby/AI/BP_Sedan_AI.MoveRight` (`self.OwnSedan AI`) _returnvalue_11)))
          (elif (> _returnvalue_yaw (- 0.0 (`KismetMathLibrary.DegAcos` _returnvalue_7)))
            (`/Game/CarDerby/AI/BP_Sedan_AI.MoveRight` (`self.OwnSedan AI`) (* _returnvalue_7 -1.0))
            (else
              (`/Game/CarDerby/AI/BP_Sedan_AI.MoveRight` (`self.OwnSedan AI`) _returnvalue_7)))))
      (else
        (`/Game/CarDerby/AI/BP_Sedan_AI.MoveRight` (`self.OwnSedan AI`) 0.0)
        (`/Game/CarDerby/AI/BP_Sedan_AI.MoveForward` (`self.OwnSedan AI`) 1.0)))))

(fn `JustMoving`)

(fn `ToggleBlock`
  (set `self.Blocked` false))

(fn `UserConstructionScript`)