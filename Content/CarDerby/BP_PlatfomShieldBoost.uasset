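; Car Derby shield pickup that grants immortality to the car that drives into it.
; On actor overlap it casts to the AI sedan first, then falls back to the player sedan, setting that car's immortal flag and showing the shield image on its HUD widget.
; The pickup destroys itself after either grant; it sets no timer and never clears the flag itself.
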(event `self.ReceiveActorBeginOverlap`
  (params (OtherActor :type "Actor Object Reference"))
  (`parent.ReceiveActorBeginOverlap` OtherActor)
  (bind _asbp_sedan_ai (cast `/Game/CarDerby/AI/BP_Sedan_AI` OtherActor)
    (:`then`
      (set `/Game/CarDerby/AI/BP_Sedan_AI.AICarImmortal?` true _asbp_sedan_ai)
      (`Widget.SetVisibility` (`/Game/CarDerby/Widgets/W_HP_and_Name.Shield_Image` (`/Game/CarDerby/AI/BP_Sedan_AI.SedanAI_W_HP_and_Name` _asbp_sedan_ai)) "Visible"))
    (:`CastFailed`
      (bind _assedan (cast `/Game/CarDerby/Sedan` OtherActor))
      (set `/Game/CarDerby/Sedan.PlayerCarImmortal?` true _assedan)
      (`Widget.SetVisibility` (`/Game/CarDerby/Widgets/W_HP_and_Name.Shield_Image` (`/Game/CarDerby/Sedan.Sedan_W_HP_and_Name` _assedan)) "Visible")))
  (`self.K2_DestroyActor`))

(fn `UserConstructionScript`
  (`parent.UserConstructionScript`))